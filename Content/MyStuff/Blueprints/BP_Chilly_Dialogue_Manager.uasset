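; Dialogue manager Blueprint for Chilly that steps through an array of lines and shows them in a dialogue widget.
; SayTheThing adds the NIWDialogue widget to the viewport, passes it the line at the current index, then calls LoadNextThingToSay.
; The LoadNextThingToSay event caches that line, increments and prints the index with no bounds check.
; A similarly named function graph and the construction script are empty.
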(event `Load Next Thing To Say`
  (bind _current_say_index (`self.Current Say Index`))
  (set `self.Current Thing To Say` (`|GetArrayItem` (`self.Things To Say`) _current_say_index))
  (bind _output_get (set `self.Current Say Index` (+ _current_say_index 1)))
  (`KismetSystemLibrary.PrintString` (`KismetStringLibrary.Conv_IntToString` _output_get)))

(event `Say The Thing`
  (bind _niw_dialogue (`self.NIW Dialogue`))
  (`UserWidget.AddToViewport` _niw_dialogue 0)
  (`/Game/MyStuff/UI/Widgets/WBP_Chilly_Dialogue.Say The Thing` _niw_dialogue (`|GetArrayItem` (`self.Things To Say`) (`self.Current Say Index`)))
  (`self.Load  Next Thing To Say`))

(fn `Load  Next Thing To Say`)

(fn `UserConstructionScript`)