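; BP_ShrinkTriggerBox is a trigger volume that toggles a BP_ShooterCharacter between shrunken and normal size.
; Begin overlap restarts the Shrink timeline, whose Finished output passes through a DoOnce that any end overlap resets.
; It then flips the character's IsShrunk flag and snaps the capsule's world scale to match, as the timeline only delays the change.
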(event `self.Shrink Trigger Box.OnComponentBeginOverlap`
  (params (OverlappedComponent :type "PrimitiveComponent Object Reference") (OtherActor :type "Actor Object Reference") (OtherComp :type "PrimitiveComponent Object Reference") (OtherBodyIndex :type Integer) (bFromSweep :type Boolean) (SweepResult :type "HitResult Structure (by ref)"))
  (`Timeline|Shrink` :!via `PlayFromStart`
    (:`Finished`
      (`/Engine/EditorBlueprintResources/StandardMacros.DoOnce` false :!label _label
        (:`Completed`
          (bind _asbp_shooter_character (cast `/Game/Variant_Shooter/Blueprints/BP_ShooterCharacter` OtherActor))
          (set `self.Character` _asbp_shooter_character)
          (if (`/Game/Variant_Shooter/Blueprints/BP_ShooterCharacter.IsShrunk` _asbp_shooter_character)
            (bind _capsulecomponent (`Character.CapsuleComponent` _asbp_shooter_character))
            (`SceneComponent.SetWorldScale3D` _capsulecomponent (1.0 1.0 1.0))
            (set `/Game/Variant_Shooter/Blueprints/BP_ShooterCharacter.IsShrunk` false _asbp_shooter_character)
            (else
              (`SceneComponent.SetWorldScale3D` _capsulecomponent (0.2 0.2 0.2))
              (set `/Game/Variant_Shooter/Blueprints/BP_ShooterCharacter.IsShrunk` true _asbp_shooter_character))))))))

(event `self.Shrink Trigger Box.OnComponentEndOverlap`
  (params (OverlappedComponent :type "PrimitiveComponent Object Reference") (OtherActor :type "Actor Object Reference") (OtherComp :type "PrimitiveComponent Object Reference") (OtherBodyIndex :type Integer))
  (goto _label :!via `Reset`))

(fn `UserConstructionScript`)